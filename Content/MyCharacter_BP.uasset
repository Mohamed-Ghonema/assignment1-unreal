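; Player character Blueprint that handles speed adjustment and camera switching.
; It enables input on BeginPlay.
; Holding speedUp or slowDown shifts the MovementSpeed variable by a fixed step, which is undone on release; the graph does not apply that variable to movement.
; Switch Cam uses a FlipFlop to toggle which of the FirstPerson and FollowCamera components is active, starting with first person on the first press.
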(event `self.ReceiveBeginPlay`
  (`self.EnableInput` null))

(event `InputAction|speedUp`
  (params (Key :type "Key Structure"))
  (:`Pressed`
    (set `self.movementSpeed` (+ (`self.movementSpeed`) 10.0)))
  (:`Released`
    (set `self.movementSpeed` (+ (`self.movementSpeed`) -10.0))))

(event `InputAction|slowDown`
  (params (Key :type "Key Structure"))
  (:`Pressed`
    (set `self.movementSpeed` (+ (`self.movementSpeed`) -10.0)))
  (:`Released`
    (set `self.movementSpeed` (+ (`self.movementSpeed`) 10.0))))

(event `InputAction|Switch Cam`
  (params (Key :type "Key Structure"))
  (:`Pressed`
    (`/Engine/EditorBlueprintResources/StandardMacros.FlipFlop`
      (:`A`
        (`ActorComponent.SetActive` (`self.first person`) true false)
        (`ActorComponent.SetActive` (`self.FollowCamera`) false false))
      (:`B`
        (`ActorComponent.SetActive` (`self.FollowCamera`) true false)
        (`ActorComponent.SetActive` (`self.first person`) false false)))))

(fn `UserConstructionScript`)